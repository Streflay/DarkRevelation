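; BP_Character1 is an FPS player character with jump input and ragdoll death.
; Shortly after BeginPlay it hides the head bone on the locally controlled mesh, and it allows jumping only when not falling.
; DeathComp's OnDeath disables capsule collision and movement, switches the mesh to physics simulation and turns off ThirdPersonMesh's hidden shadow.
; GetPlayerRef returns the character itself.
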(event `self.ReceiveBeginPlay`
  (`KismetSystemLibrary.Delay` 0.01)
  (if (`self.IsLocallyControlled`)
    (`SkinnedMeshComponent.HideBoneByName` (`self.Mesh`) "head" "PBO_None")))

(event `EnhancedInput|/Game/FPSAction/Input/Input_Jump`
  (params (ActionValue :type Boolean) (ElapsedSeconds :type "Float (double-precision)") (TriggeredSeconds :type "Float (double-precision)") (InputAction :type "InputAction Object Reference" :default "/Game/FPSAction/Input/Input_Jump.Input_Jump"))
  (:`Triggered`
    (if (`self.f_IsNot_Jumping`)
      (`self.Jump`))))

(event `self.DeathComp.OnDeath`
  (bind _mesh (`self.Mesh`))
  (`PrimitiveComponent.SetCollisionEnabled` (`self.CapsuleComponent`) "NoCollision")
  (`PrimitiveComponent.SetCollisionEnabled` _mesh "PhysicsOnly")
  (`PrimitiveComponent.SetSimulatePhysics` _mesh true)
  (`SkeletalMeshComponent.PlayAnimation` _mesh null false)
  (`CharacterMovementComponent.DisableMovement` (`self.CharacterMovement`))
  (`PrimitiveComponent.SetCastHiddenShadow` (`self.ThirdPersonMesh`) false))

(fn `f_IsNot_Jumping`
  (returns (ReturnValue :type Boolean))
  (return (not (`NavMovementInterface.IsFalling` (`self.CharacterMovement`)))))

(fn `Get Player Ref`
  (returns (Player :type "FPSCharacter Object Reference"))
  (return self))

(fn `UserConstructionScript`)